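; Example flammable particle-effect actor in the wind system that starts burning on BeginPlay and can spread fire to other actors.
; FireOn and FireOff toggle the particle system's visibility and the IsOnFire flag, with the construction script applying the Emitter template.
; While burning, its Box overlap calls FireOn on actors implementing Interface_Flammable.
; Fire spreading is marked experimental, and spread fires currently receive no wind.
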(event `self.Box.OnComponentBeginOverlap`
  (params (OverlappedComponent :type "PrimitiveComponent Object Reference") (OtherActor :type "Actor Object Reference") (OtherComp :type "PrimitiveComponent Object Reference") (OtherBodyIndex :type Integer) (bFromSweep :type Boolean) (SweepResult :type "HitResult Structure (by ref)"))
  ;[1 1 1] spread fire (experimental) spread fires currently do not receive winds
  (set `self.OtherActor` OtherActor)
  (if (and (`KismetSystemLibrary.DoesImplementInterface` OtherActor "/Game/WindSystem/Blueprints/Interfaces/Interface_Flammable.Interface_Flammable_C") (`self.IsOnFire`))
    (message `/Game/WindSystem/Blueprints/Interfaces/Interface_Flammable.FireOn` (`self.OtherActor`))))

(event `/Game/WindSystem/Blueprints/Interfaces/Interface_Flammable.FireOn`
  ;[1 1 1] Set fire on off
  (`SceneComponent.SetVisibility` (`self.ParticleSystem`) true false)
  (set `self.IsOnFire` true))

(event `/Game/WindSystem/Blueprints/Interfaces/Interface_Flammable.FireOff`
  ;[1 1 1] Set fire on off
  (`SceneComponent.SetVisibility` (`self.ParticleSystem`) false false)
  (set `self.IsOnFire` false))

(event `self.ReceiveBeginPlay`
  (`self.FireOn`))

(fn `UserConstructionScript`
  (`ParticleSystemComponent.SetTemplate` (`self.ParticleSystem`) (`self.Emitter`)))