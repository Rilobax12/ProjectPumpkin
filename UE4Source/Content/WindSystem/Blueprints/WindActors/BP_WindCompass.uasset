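; BP_WindCompass is a wind indicator actor that shows the speed and direction of the wind zone in the level.
; One second after BeginPlay it caches the first BP_WindZoneBase actor it finds.
; Each tick it turns the text toward the player camera and displays WindSpeed, while the arrow copies WindRotation and stretches along X with speed, clamped between 1 and 1.5.
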(event `self.ReceiveBeginPlay`
  ;[1 1 1] get  windzone
  (`KismetSystemLibrary.Delay` 1.0)
  (bind _outactors (`GameplayStatics.GetAllActorsOfClass` "/Game/WindSystem/Blueprints/BaseClasses/BP_WindZoneBase.BP_WindZoneBase_C"))
  (set `self.CurrentWindzone` (`KismetArrayLibrary.Array_Get` _outactors)))

(event `self.ReceiveTick`
  (params (DeltaSeconds :type "Float (single-precision)"))
  (bind _currentwindzone (`self.CurrentWindzone`))
  (bind _currentwindzone_2 (`self.CurrentWindzone`))
  (`|ExecutionSequence`
    (:`then_0`
      ;[1 1 1] rotate text to cam
      (`SceneComponent.K2_SetWorldRotation` (`self.TextRender`) (`KismetMathLibrary.FindLookAtRotation` (`SceneComponent.K2_GetComponentLocation` (`self.TextRender`)) (`PlayerCameraManager.GetCameraLocation` (`GameplayStatics.GetPlayerCameraManager` 0))) false false)
      ;[1 1 1] update text
      (`/Engine/EditorBlueprintResources/StandardMacros.IsValid` _currentwindzone_2
        (:`Is Valid`
          (`TextRenderComponent.K2_SetText` (`self.TextRender`) (`KismetTextLibrary.Conv_DoubleToText` (`/Game/WindSystem/Blueprints/BaseClasses/BP_WindZoneBase.WindSpeed` _currentwindzone_2) "HalfToEven" true 1 324 0 1)))))
    (:`then_1`
      (`/Engine/EditorBlueprintResources/StandardMacros.IsValid` _currentwindzone
        (:`Is Valid`
          (`SceneComponent.SetWorldScale3D` (`self.Arrow`) (`KismetMathLibrary.MakeVector` (`KismetMathLibrary.MapRangeClamped` (`/Game/WindSystem/Blueprints/BaseClasses/BP_WindZoneBase.WindSpeed` _currentwindzone) 0.0 1.0 1.0 1.5) 1.0 1.0))
          (`SceneComponent.K2_SetWorldRotation` (`self.Arrow`) (`/Game/WindSystem/Blueprints/BaseClasses/BP_WindZoneBase.WindRotation` (`self.CurrentWindzone`)) false false))))))

(fn `UserConstructionScript`)