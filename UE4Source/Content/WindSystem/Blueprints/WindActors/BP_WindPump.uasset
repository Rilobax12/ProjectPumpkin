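; BP_WindPump is a wind pump actor that animates in response to the wind system.
; The construction script caches the first BP_WindZoneBase actor found as its active wind zone.
; Each tick sets the tail's relative yaw to that zone's wind direction and rolls the wings by an ease-out curve of offset wind speed.
; The wing rotation is added per frame without delta-time scaling, so spin rate depends on frame rate.
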(event `self.ReceiveTick`
  (params (DeltaSeconds :type "Float (single-precision)"))
  (`|ExecutionSequence`
    (:`then_0`
      ;[1 1 1] rotate tail
      (`SceneComponent.K2_SetRelativeRotation` (`self.SM_Helper_Windpump_Tail`) (`KismetMathLibrary.MakeRotator` 0.0 0.0 (.yaw (`/Game/WindSystem/Blueprints/BaseClasses/BP_WindZoneBase.WindRotation` (`self.ActiveWindZone`)))) false false))
    (:`then_1`
      ;[1 1 1] rotate tail
      (`SceneComponent.K2_AddRelativeRotation` (`self.SM_Helper_Windpump_Wings`) (`KismetMathLibrary.MakeRotator` (`|EaseFunction` "EaseOut" (+ (`/Game/WindSystem/Blueprints/BaseClasses/BP_WindZoneBase.WindSpeed` (`self.ActiveWindZone`)) 0.2) 0.0 1.0 3.0)) false false))))

(fn `UserConstructionScript`
  (bind _outactors (`GameplayStatics.GetAllActorsOfClass` "/Game/WindSystem/Blueprints/BaseClasses/BP_WindZoneBase.BP_WindZoneBase_C"))
  (bind _item (`KismetArrayLibrary.Array_Get` _outactors))
  (`/Engine/EditorBlueprintResources/StandardMacros.IsValid` _item
    (:`Is Valid`
      (set `self.ActiveWindZone` _item))))