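; Example fabric actor for the wind system that drives its looping flag sound from the local wind speed.
; On BeginPlay it finds wind zone actors overlapping its static mesh and stores the last one as its wind zone.
; Each tick, while that zone is valid, it feeds the zone's WindSpeed into the audio component's RollSpeed parameter, intended to control flag volume.
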(event `self.ReceiveBeginPlay`
  ;[1 1 1] get windzone
  (for _array_element (`PrimitiveComponent.GetOverlappingActors` (`self.StaticMesh`) "/Game/WindSystem/Blueprints/BaseClasses/BP_WindZoneBase.BP_WindZoneBase_C")
    (bind _asbp_wind_zone_base (cast `/Game/WindSystem/Blueprints/BaseClasses/BP_WindZoneBase` _array_element))
    (set `self.Windzone` _asbp_wind_zone_base)))

(event `self.ReceiveTick`
  (params (DeltaSeconds :type "Float (single-precision)"))
  (bind _windzone (`self.Windzone`))
  ;[1 1 1] set flag audio volume based on windspeed
  (`/Engine/EditorBlueprintResources/StandardMacros.IsValid` _windzone
    (:`Is Valid`
      (`AudioComponent.SetFloatParameter` (`self.S_SFX_Flag_Loop_1`) "RollSpeed" (`/Game/WindSystem/Blueprints/BaseClasses/BP_WindZoneBase.WindSpeed` _windzone)))))

(fn `UserConstructionScript`)