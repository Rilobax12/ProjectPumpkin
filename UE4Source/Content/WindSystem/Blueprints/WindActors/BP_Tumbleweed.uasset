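; BP_Tumbleweed is a wind-driven, flammable tumbleweed prop that initializes a WindComponent with its mesh and audio.
; The construction script optionally randomizes squeeze, scale and rotation, then lifts the mesh out of the ground.
; BeginPlay caches the overlapping wind zone and ignites if flagged.
; Ignition attaches fire and audio once, registers the emitter with that zone, and lets sphere overlaps spread fire through Interface_Flammable.
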(event `/Game/WindSystem/Blueprints/Interfaces/Interface_Flammable.FireOn`
  ;[1 1 1] Fire event
  (`self.SpawnFire`))

(event `self.Sphere.OnComponentBeginOverlap`
  (params (OverlappedComponent :type "PrimitiveComponent Object Reference") (OtherActor :type "Actor Object Reference") (OtherComp :type "PrimitiveComponent Object Reference") (OtherBodyIndex :type Integer) (bFromSweep :type Boolean) (SweepResult :type "HitResult Structure (by ref)"))
  ;[1 1 1] spread fire to another flammable object
  (set `self.OtherActor` OtherActor)
  (if (and (`self.IsOnFire`) (`KismetSystemLibrary.DoesImplementInterface` (`self.OtherActor`) "/Game/WindSystem/Blueprints/Interfaces/Interface_Flammable.Interface_Flammable_C"))
    (message `/Game/WindSystem/Blueprints/Interfaces/Interface_Flammable.FireOn` (`self.OtherActor`))))

(event `self.ReceiveBeginPlay`
  ;[1 1 1] set tumblers manually on fire by public bool
  (bind _asbp_wind_zone_base (cast `/Game/WindSystem/Blueprints/BaseClasses/BP_WindZoneBase` (`KismetArrayLibrary.Array_Get` (`PrimitiveComponent.GetOverlappingActors` (`self.Sphere`) "/Game/WindSystem/Blueprints/BaseClasses/BP_WindZoneBase.BP_WindZoneBase_C"))))
  (set `self.CurrentWindZone` _asbp_wind_zone_base)
  (if (`self.IsOnFire`)
    (`self.FireOn`)))

(fn `SpawnFire`
  (bind _currentwindzone (`self.CurrentWindZone`))
  ;[1 1 1] FireSpawn when there isn't already a fire
  (`/Engine/EditorBlueprintResources/StandardMacros.IsValid` (`self.AttachedFireEmitter`)
    (:`Is Not Valid`
      (bind _returnvalue (`GameplayStatics.SpawnEmitterAttached` "/Game/WindSystem/StarterContentFire/Particles/P_Fire.P_Fire" (`self.StaticMesh`) "None" (0.0 0.0 0.0) (struct) "SnapToTarget"))
      (set `self.AttachedFireEmitter` _returnvalue)
      (set `self.IsOnFire` true)
      (`AddComponent|NODE_AddAudioComponent-0` :`bManualAttachment` true :`RelativeTransform` (`SceneComponent.GetRelativeTransform` (`self.StaticMesh`)))
      (`/Engine/EditorBlueprintResources/StandardMacros.IsValid` _currentwindzone
        (:`Is Valid`
          (`KismetArrayLibrary.Array_AddUnique` (`/Game/WindSystem/Blueprints/BaseClasses/BP_WindZoneBase.ReceivedParticles` _currentwindzone) (`self.AttachedFireEmitter`)))))))

(fn `UserConstructionScript`
  (bind _returnvalue (`KismetMathLibrary.RandomFloatInRange` 0.0 180.0))
  (`/Game/WindSystem/Blueprints/Components/BP_WindComponent.InitializeWindComponent` (`self.WindComponent`) (`self.Audio`) (`self.StaticMesh`))
  ;[1 1 1] Set randomized scale and rotation around z when placing actors
  (if (`self.UseRandomization`)
    (`SceneComponent.SetWorldScale3D` (`self.StaticMesh`) (* (`KismetMathLibrary.MakeVector` 1.0 1.0 (- 1.0 (`KismetMathLibrary.RandomFloatInRange` 0.0 (`self.RandomSqueezeFactorMax`)))) (`KismetMathLibrary.RandomFloatInRange` (`self.RandomScaleMin`) (`self.RandomScaleMax`))))
    (`SceneComponent.K2_SetRelativeRotation` (`self.StaticMesh`) (`KismetMathLibrary.MakeRotator` _returnvalue _returnvalue _returnvalue) false false)
    ;[1 1 1] prevent placing inside of ground geometry
    (`SceneComponent.K2_SetRelativeLocation` (`self.StaticMesh`) (`KismetMathLibrary.MakeVector` (.x (`SceneComponent.RelativeLocation` (`self.StaticMesh`))) (.y (`SceneComponent.RelativeLocation` (`self.StaticMesh`))) (+ (.z (`SceneComponent.RelativeLocation` (`self.StaticMesh`))) (/ (.z (`.BoxExtent` (`self.GetActorBounds` false))) 2.0))) false false)))