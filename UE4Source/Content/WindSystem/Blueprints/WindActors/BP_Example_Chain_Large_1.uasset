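; Example wind actor from the WindSystem: a large chain made of four link components, set up through a wind component.
; The construction script initializes BPWindComponent with the first link as its mesh, along with an audio component.
; It then copies the component's angular and linear damping to all four links, as a custom step for non-randomized transform actions.
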(fn `UserConstructionScript`
  (`/Game/WindSystem/Blueprints/Components/BP_WindComponent.InitializeWindComponent` (`self.BP_WindComponent`) (`self.Audio`) (`self.Link1`))
  ;[1 1 1] Customization of construction script for non randomized transform actions
  ;;[1 1 1] set dampings
  (`PrimitiveComponent.SetAngularDamping` (`self.Link1`) (`/Game/WindSystem/Blueprints/Components/BP_WindComponent.AngularDamping` (`self.BP_WindComponent`)))
  (`PrimitiveComponent.SetAngularDamping` (`self.Link3`) (`/Game/WindSystem/Blueprints/Components/BP_WindComponent.AngularDamping` (`self.BP_WindComponent`)))
  (`PrimitiveComponent.SetAngularDamping` (`self.Link4`) (`/Game/WindSystem/Blueprints/Components/BP_WindComponent.AngularDamping` (`self.BP_WindComponent`)))
  (`PrimitiveComponent.SetAngularDamping` (`self.Link2`) (`/Game/WindSystem/Blueprints/Components/BP_WindComponent.AngularDamping` (`self.BP_WindComponent`)))
  (`PrimitiveComponent.SetLinearDamping` (`self.Link1`) (`/Game/WindSystem/Blueprints/Components/BP_WindComponent.LinearDamping` (`self.BP_WindComponent`)))
  (`PrimitiveComponent.SetLinearDamping` (`self.Link3`) (`/Game/WindSystem/Blueprints/Components/BP_WindComponent.LinearDamping` (`self.BP_WindComponent`)))
  (`PrimitiveComponent.SetLinearDamping` (`self.Link4`) (`/Game/WindSystem/Blueprints/Components/BP_WindComponent.LinearDamping` (`self.BP_WindComponent`)))
  (`PrimitiveComponent.SetLinearDamping` (`self.Link2`) (`/Game/WindSystem/Blueprints/Components/BP_WindComponent.LinearDamping` (`self.BP_WindComponent`))))