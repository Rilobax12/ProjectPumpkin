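; Base wind zone actor that simulates changing wind for physics meshes, particles, cloth and foliage.
; Tick samples randomly chosen speed curves and drives a sound parameter, while a looping timeline randomizes direction.
; ApplyForce, run per registered actor, pushes simulating meshes and updates particle parameters, a child WindDirectionalSource and the grass shader's parameter collection.
; Construction warns about multiple zones and can scatter seeded, line-traced child actors inside a box.
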(event `PFXCollector`
  (`|ExecutionSequence`
    (:`then_0`
      ;[1 1 1] get emitters inside actors
      (bind _outactors (`GameplayStatics.GetAllActorsOfClass` "/Script/Engine.Actor"))
      (for _array_element _outactors
        (`KismetArrayLibrary.Array_AddUnique` (`self.ReceivedParticles`) (`self.GetComponentByClass` _array_element "/Script/Engine.ParticleSystemComponent"))))
    (:`then_1`
      ;[1 1 1] get directly placed emitters
      (bind _outactors_2 (`GameplayStatics.GetAllActorsOfClass` "/Script/Engine.Emitter"))
      (for _array_element_2 _outactors_2
        (`KismetArrayLibrary.Array_AddUnique` (`self.ReceivedParticles`) (`Emitter.ParticleSystemComponent` _array_element_2))))))

(event `self.ReceiveBeginPlay`
  ;[1 1 1] Call custom events at begin play
  (`|ExecutionSequence`
    (:`then_0`
      (`self.AddClothWindsource`))
    (:`then_1`
      (`self.SelectWindcurves`))
    (:`then_2`
      (`self.PFXCollector`))
    (:`then_4`
      ;;[1 1 1] windspeed of wind directional source is only updated when source is rotated. therefore must rotate forever
      (`self.ChangeWinddirection`))))

(event `AddClothWindsource`
  ;[1 1 1] Add a wind directional source component to affect physx cloth objects
  (bind _returnvalue (`AddComponent|NODE_AddChildActorComponent-0`))
  (`/Engine/EditorBlueprintResources/StandardMacros.IsValid` _returnvalue
    (:`Is Valid`
      (bind _aswind_directional_source (cast `WindDirectionalSource` (`ChildActorComponent.ChildActor` _returnvalue)))
      (set `self.WindSource` (`WindDirectionalSource.Component` _aswind_directional_source))
      (`KismetSystemLibrary.Delay` 1.0)
      (`WindDirectionalSourceComponent.SetStrength` (`self.WindSource`) 1.0)
      (`WindDirectionalSourceComponent.SetSpeed` (`self.WindSource`) (* (`self.WindSpeed`) (`self.ClothWindMultiplier`))))))

(event `ChangeWinddirection`
  ;[1 1 1] Random wind direction
  ;;[1 1 1] ChangeWindDirection
  (set `self.WindDirection` (`KismetMathLibrary.MakeRotator` 0.0 0.0 (+ (.yaw (`self.OldWindDirection`)) (`KismetMathLibrary.RandomFloatInRange` (`self.MinWindDirectionChange`) (`self.MaxWindDirectionChange`)))))
  (bind (_direction _0_1) (`Timeline|WindDirectionLerpAlpha` :!via `PlayFromStart`)
    (:`Update`
      (bind _returnvalue (`KismetMathLibrary.RLerp` (`self.OldWindDirection`) (`self.WindDirection`) _0_1))
      (`SceneComponent.K2_SetWorldRotation` (`self.WindSource`) _returnvalue false false)
      (set `self.WindRotation` _returnvalue))
    (:`Finished`
      (set `self.OldWindDirection` (`self.WindDirection`))
      (`self.ChangeWinddirection`))))

(event `SelectWindcurves`
  (bind _windsound (`self.WindSound`))
  ;[1 1 1] Handle wind curve selection (implement GetTimeRange)
  ;;[1 1 1] select a random windcurve
  (set `self.ActiveCurveIndex` (`KismetMathLibrary.RandomIntegerInRange` 0 (- (`KismetArrayLibrary.Array_Length` (`self.WindCurves`)) 1)))
  (`/Engine/EditorBlueprintResources/StandardMacros.IsValid` _windsound
    (:`Is Valid`
      (bind _returnvalue (`GameplayStatics.SpawnSound2D` _windsound))
      (`/Engine/EditorBlueprintResources/StandardMacros.IsValid` _returnvalue
        (:`Is Valid`
          (set `self.WindSoundCue` _returnvalue))))))

(event `PlayNewCurve`
  (bind _activecurvetime (`self.ActiveCurveTime`))
  (bind _output (`|GetArrayItem` (`self.WindCurves`) (`self.ActiveCurveIndex`)))
  ;[1 1 1] Handle wind curve selection (implement GetTimeRange)
  (bind _output_get (set `self.WindSpeed` (* (`CurveFloat.GetFloatValue` _output _activecurvetime) (`self.PhysicalWindMultiplier`)) :!label _label))
  ;;[1 1 1] is current windcurve still acting
  (if (not (`KismetMathLibrary.NearlyEqual_FloatFloat` (`.MaxTime` (`CurveBase.GetTimeRange` _output)) _activecurvetime 0.2))
    ;;[1 1 1] calculates new time
    (set `self.ActiveCurveTime` (+ (`self.ActiveCurveTime`) (`GameplayStatics.GetWorldDeltaSeconds`)))
    (else
      ;;[1 1 1] picks a new windcurve
      (set `self.ActiveCurveIndex` (`KismetMathLibrary.RandomIntegerInRange` 0 (- (`KismetArrayLibrary.Array_Length` (`self.WindCurves`)) 1)))
      ;;[1 1 1] resets the time
      (set `self.ActiveCurveTime` 0.0)
      (`self.PlayNewCurve`))))

(event `self.ReceiveTick`
  (params (DeltaSeconds :type "Float (single-precision)"))
  (bind _windsoundcue (`self.WindSoundCue`))
  (`|ExecutionSequence`
    (:`then_0`
      (goto _label))
    (:`then_1`
      ;[1 1 1] for each wind affected actor
      (for _array_element (`self.ReceivedParticles`)
        (bind _output_get (set `self.CurrentAffectedPFX` _array_element))
        ;[1 1 1] check if it's still valid
        (`/Engine/EditorBlueprintResources/StandardMacros.IsValid` _output_get
          (:`Is Not Valid`
            ;[1 1 1] remove from list
            (`KismetArrayLibrary.Array_RemoveItem` (`self.ReceivedParticles`) (`self.CurrentAffectedPFX`))))))
    (:`then_2`
      (for _array_element_2 (`self.ReceivedStandardActors`)
        (bind _output_get_2 (set `self.CurrentAffectedActor` _array_element_2))
        (`/Engine/EditorBlueprintResources/StandardMacros.IsValid` _output_get_2
          (:`Is Valid`
            ;[1 1 1] send to custom event
            (`self.ApplyForce`))
          (:`Is Not Valid`
            (`KismetArrayLibrary.Array_RemoveItem` (`self.ReceivedStandardActors`) (`self.CurrentAffectedActor`))))))
    (:`then_3`
      ;[1 1 1] set wind sound parameter
      (`/Engine/EditorBlueprintResources/StandardMacros.IsValid` _windsoundcue
        (:`Is Valid`
          (`AudioComponent.SetFloatParameter` _windsoundcue "Speed" (/ (`self.WindSpeed`) (`self.PhysicalWindMultiplier`))))))
    (:`then_4`
      (`self.WarningTextRotate`))))

(event `ApplyForce`
  ;[1 1 1] Apply winds
  (set `self.CurrentWindActorForce` (`self.ComputeWindload` (* (`/Game/WindSystem/Blueprints/Components/BP_WindComponent.EstimatedSurfaceArea` (`self.GetComponentByClass` (`self.CurrentAffectedActor`) "/Game/WindSystem/Blueprints/Components/BP_WindComponent.BP_WindComponent_C")) 10000.0) (`self.WindSpeed`)))
  (`|ExecutionSequence`
    (:`then_0`
      ;;[1 1 1] apply windloadforce
      (for _array_element (`self.K2_GetComponentsByClass` (`self.CurrentAffectedActor`) "/Script/Engine.StaticMeshComponent")
        (bind _asstatic_mesh_component (cast `StaticMeshComponent` _array_element))
        (if (`SceneComponent.IsAnySimulatingPhysics` _asstatic_mesh_component)
          (`PrimitiveComponent.AddForce` _asstatic_mesh_component (`self.CurrentWindActorForce`) "None" false))))
    (:`then_1`
      ;;[1 1 1] set particle acceleration based on windforce
      (for _array_element_2 (`self.ReceivedParticles`)
        (`/Engine/EditorBlueprintResources/StandardMacros.IsValid` _array_element_2
          (:`Is Valid`
            (`ParticleSystemComponent.SetVectorParameter` _array_element_2 "wind" (`KismetMathLibrary.GreaterGreater_VectorRotator` (`KismetMathLibrary.MakeVector` (* (`self.WindSpeed`) (`self.ParticleWindMultiplier`))) (`self.WindRotation`)))))))
    (:`then_2`
      ;;[1 1 1] add force to cloth; communication with wind directional sources is limited.
      (`/Engine/EditorBlueprintResources/StandardMacros.IsValid` (`self.WindSource`)
        (:`Is Valid`
          (`WindDirectionalSourceComponent.SetSpeed` (`self.WindSource`) (`KismetMathLibrary.MapRangeClamped` (* (`self.WindSpeed`) (`self.ClothWindMultiplier`)) 0.0 4.0 0.0 1.0)))))
    (:`then_3`
      ;;[1 1 1] hand wind speed to the parameter collection. this is used by the grass shader
      (`KismetMaterialLibrary.SetVectorParameterValue` "/Game/WindSystem/Materials/ParameterCollections/PC_WindDirection.PC_WindDirection" "WindDirection" (`KismetMathLibrary.Conv_VectorToLinearColor` (`KismetMathLibrary.GreaterGreater_VectorRotator` (`KismetMathLibrary.MakeVector` (* (`self.WindSpeed`) (`self.FoliageWindMultiplier`))) (`self.WindRotation`)))))))

(event `WarningTextRotate`
  (bind _textrender (`self.TextRender`))
  ;[1 1 1] rotate warning text to player cam
  (if (`SceneComponent.IsVisible` _textrender)
    (`SceneComponent.K2_SetWorldRotation` (`self.TextRender`) (`KismetMathLibrary.FindLookAtRotation` (`SceneComponent.K2_GetComponentLocation` _textrender) (`PlayerCameraManager.GetCameraLocation` (`GameplayStatics.GetPlayerCameraManager` 0))) false false)))

(fn `UserConstructionScript`
  (bind _actorstobespawned (`self.ActorsToBeSpawned`))
  (bind _onlyspawnonspecificclasses (`self.OnlySpawnOnSpecificClasses`))
  (bind _spawnzone (`self.SpawnZone`))
  (bind _returnvalue (`SceneComponent.K2_GetComponentRotation` _spawnzone))
  (bind _x (.x (`BoxComponent.GetScaledBoxExtent` (`self.SpawnZone`))))
  (bind _y (.y (`BoxComponent.GetScaledBoxExtent` (`self.SpawnZone`))))
  (bind _z (.z (`BoxComponent.GetScaledBoxExtent` (`self.SpawnZone`))))
  (bind _returnvalue_2 (`KismetMathLibrary.MakeVector` (`KismetMathLibrary.RandomFloatInRangeFromStream` (* _x -1.0) _x (`self.RandomStream`)) (`KismetMathLibrary.RandomFloatInRangeFromStream` (* _y -1.0) _y (`self.RandomStream`)) _z))
  (bind _returnvalue_3 (`KismetMathLibrary.GreaterGreater_VectorRotator` (+ _returnvalue_2 (`SceneComponent.K2_GetComponentLocation` _spawnzone)) _returnvalue))
  ;[1 1 1] warning when more than one windzone is placed
  (bind _outactors (`GameplayStatics.GetAllActorsOfClass` "BP_WindZoneBase_C"))
  (if (`KismetArrayLibrary.Array_IsValidIndex` _outactors)
    (`SceneComponent.SetVisibility` (`self.TextRender`) (> (`KismetArrayLibrary.Array_Length` _outactors) 1) false)
    ;[1 1 1] make custom editor sprite
    (set `BillboardComponent.Sprite` "/Engine/EditorResources/S_WindDirectional.S_WindDirectional" (`self.Billboard`))
    ;[1 1 1] set the sound cue
    (`/Engine/EditorBlueprintResources/StandardMacros.IsValid` (`self.WindSoundCue`)
      (:`Is Valid`
        (`/Engine/EditorBlueprintResources/StandardMacros.IsValid` (`self.WindSound`)
          (:`Is Valid`
            (`AudioComponent.SetSound` (`self.WindSoundCue`) (`self.WindSound`)))
          (:`Is Not Valid`
            _)))
      (:`Is Not Valid`
        _))
    ;[1 1 1] should the zone spawn wind affected actors
    (if (`self.SpawnWindActors`)
      ;[1 1 1] make random stream
      (set `self.RandomStream` (`KismetMathLibrary.MakeRandomStream` (`self.RandomSeed`)))
      ;[1 1 1] define number of wind actors
      (for _ (range 1 (+ (`self.ActorAmount`) 1))
        ;[1 1 1] do linetrace from top of bounding box to bottom
        (bind _outhit (`KismetSystemLibrary.LineTraceSingle` :`Start` _returnvalue_3 :`End` (+ _returnvalue_3 (`KismetMathLibrary.GreaterGreater_VectorRotator` (`KismetMathLibrary.MakeVector` (.x (/ _returnvalue_2 1000.0)) (.y (/ _returnvalue_2 1000.0)) (* _z -2.0)) _returnvalue)) :`TraceChannel` "TraceTypeQuery1" :`DrawDebugType` "ForOneFrame" :`DrawTime` 1.0))
        (bind (_bblockinghit _binitialoverlap _time _distance _location _impactpoint _normal _impactnormal _physmat _hitactor) (`GameplayStatics.BreakHitResult` _outhit))
        (set `self.SpawnImpactPoint` _location)
        ;[1 1 1] prevent placing on other than defined surfaces
        (for _array_element (`self.SpawnOnObjectClasses`)
          (if (or (and (== _array_element (`GameplayStatics.GetObjectClass` _hitactor)) _onlyspawnonspecificclasses) (not _onlyspawnonspecificclasses))
            ;[1 1 1] add a child actor at trace impact
            (bind _returnvalue_4 (`AddComponent|NODE_AddChildActorComponent-1` :`bManualAttachment` true :`RelativeTransform` (`KismetMathLibrary.MakeTransform` (`self.SpawnImpactPoint`) (`KismetMathLibrary.MakeRotator` 0.0 0.0 (.yaw (`KismetMathLibrary.RandomRotator` false))))))
            (bind _output_get (set `self.NewChildActor` _returnvalue_4))
            (`KismetArrayLibrary.Array_AddUnique` (`self.AllSpawnedActors`) _output_get)
            (`ChildActorComponent.SetChildActorClass` (`self.NewChildActor`) (`|GetArrayItem` _actorstobespawned (`KismetMathLibrary.RandomIntegerInRange` 0 (`KismetArrayLibrary.Array_LastIndex` _actorstobespawned)))))))
      (else
        (for _array_element_2 (`self.AllSpawnedActors`)
          (`ActorComponent.K2_DestroyComponent` _array_element_2))))))