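; Vertical door actor that unlocks and raises when its Open event is called.
; Open caches the world locations of both locks and the door, then a timeline slides the locks in opposite directions along the actor's forward axis.
; When that finishes, a second timeline lifts the door along the actor's up vector.
; The file contains no closing logic.
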(event `Open`
  (set `self.CurrentLocLeft` (`SceneComponent.K2_GetComponentLocation` (`self.LockLeft`)))
  (set `self.CurrentLocRight` (`SceneComponent.K2_GetComponentLocation` (`self.LockRight`)))
  (set `self.CurrentLocDoor` (`SceneComponent.K2_GetComponentLocation` (`self.Door`)))
  (bind (_direction _distance) (`Timeline|LockersAnim` :!via `PlayFromStart`)
    (:`Update`
      (`SceneComponent.K2_SetWorldLocation` (`self.LockLeft`) (+ (`self.CurrentLocLeft`) (* (`self.GetActorForwardVector`) _distance)) false false)
      (`SceneComponent.K2_SetWorldLocation` (`self.LockRight`) (+ (`self.CurrentLocRight`) (* (`self.GetActorForwardVector`) (* _distance -1.0))) false false))
    (:`Finished`
      (bind (_direction_2 _distance_2) (`Timeline|DoorAnim` :!via `PlayFromStart`)
        (:`Update`
          (`SceneComponent.K2_SetWorldLocation` (`self.Door`) (+ (`self.CurrentLocDoor`) (* (`self.GetActorUpVector`) _distance_2)) false false))))))

(event `self.ReceiveBeginPlay`)

(fn `UserConstructionScript`)