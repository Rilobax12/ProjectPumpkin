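; BP_GateLocker is a destructible gate lock that breaks after taking enough point damage.
; Point damage reduces Health until it reaches zero, which sets the Break flag once and fires the OnBreak dispatcher.
; Breaking swaps in the broken mesh, enables physics simulation on it, and plays the LightOff timeline to fade the material's emissive strength to zero.
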(event `self.ReceivePointDamage`
  (params (Damage :type "Float (single-precision)") (DamageType :type "DamageType Object Reference") (HitLocation :type "Vector Structure") (HitNormal :type "Vector Structure") (HitComponent :type "PrimitiveComponent Object Reference") (BoneName :type Name) (ShotFromDirection :type "Vector Structure") (InstigatedBy :type "Controller Object Reference") (DamageCauser :type "Actor Object Reference") (HitInfo :type "HitResult Structure (by ref)"))
  (bind _gatelocker (`self.GateLocker`))
  ;[1 1 1] Is Break?
  (if (not (`self.Break`))
    ;[1 1 1] Health
    (bind _output_get (set `self.Health` (- (`self.Health`) Damage)))
    (if (<= _output_get 0.0)
      (set `self.Break` true)
      (`self.OnBreak`)
      ;[1 1 1] Death Event
      (`StaticMeshComponent.SetStaticMesh` _gatelocker "/Game/Interaction/Props/GateLocker/Meshes/SM_GateLockerBreak.SM_GateLockerBreak")
      (`PrimitiveComponent.SetSimulatePhysics` _gatelocker true)
      (bind (_direction _alpha) (`Timeline|LightOff` :!via `PlayFromStart`)
        (:`Update`
          (`MeshComponent.SetScalarParameterValueOnMaterials` (`self.GateLocker`) "Emissive Strength" (`KismetMathLibrary.Lerp` 5.0 0.0 _alpha)))))))

(fn `UserConstructionScript`)