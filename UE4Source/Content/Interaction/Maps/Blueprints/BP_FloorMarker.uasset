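; BP_FloorMarker is a floor marker actor that gives visual and audio feedback when told it is overlapped or no longer overlapped.
; BeginPlay creates a dynamic material instance from M_FloorMarker on the FloorMarker component.
; The OnOverlap event plays a different sound for each state, stops the opposing timeline and restarts its own.
; The on timeline drives overlap alpha and emissive parameters, while the off timeline drives only alpha.
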(event `self.ReceiveBeginPlay`
  ;[1 1 1] Create Matrial Instance For Dynamic
  (bind _returnvalue (`PrimitiveComponent.CreateDynamicMaterialInstance` (`self.FloorMarker`) 0 "/Game/Interaction/Props/FloorMarker/Materials/M_FloorMarker.M_FloorMarker"))
  (set `self.FloorMarkerMat` _returnvalue))

(event `OnOverlap`
  (params (Overlap :type Boolean))
  (bind _floormarkermat (`self.FloorMarkerMat`))
  (if Overlap
    (`GameplayStatics.PlaySoundAtLocation` "/Engine/VREditor/Sounds/VR_close_Cue.VR_close_Cue" (`self.K2_GetActorLocation`))
    (`TimelineComponent.Stop` (`self.OverlapPoints_Off`))
    (bind (_direction _alpha _emissive) (`Timeline|OverlapPoints_On` :!via `PlayFromStart`)
      (:`Update`
        (`MaterialInstanceDynamic.SetScalarParameterValue` _floormarkermat "OverlapAlpha" _alpha)
        (`MaterialInstanceDynamic.SetScalarParameterValue` _floormarkermat "Emissive_Overlap" _emissive)))
    (else
      (`GameplayStatics.PlaySoundAtLocation` "/Engine/VREditor/Sounds/VR_click3_Cue.VR_click3_Cue" (`self.K2_GetActorLocation`))
      (`TimelineComponent.Stop` (`self.OverlapPoints_On`))
      (bind (_direction_2 _alpha_2) (`Timeline|OverlapPoints_Off` :!via `PlayFromStart`)
        (:`Update`
          (`MaterialInstanceDynamic.SetScalarParameterValue` (`self.FloorMarkerMat`) "OverlapAlpha" _alpha_2))))))

(fn `UserConstructionScript`)