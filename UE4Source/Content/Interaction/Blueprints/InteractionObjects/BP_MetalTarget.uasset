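; BP_MetalTarget is a shootable target with two physics-constrained chains that scores point damage by accuracy.
; Hits on the Target component earn points by distance from its world location and pass them to CallTargetHit.
; HitPoints uses nested distance bands, where a repeated threshold makes the 4-point band unreachable.
; Other hits go to Chains, which breaks the physics constraint matching the struck left or right link.
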(event `self.ReceivePointDamage`
  (params (Damage :type "Float (single-precision)") (DamageType :type "DamageType Object Reference") (HitLocation :type "Vector Structure") (HitNormal :type "Vector Structure") (HitComponent :type "PrimitiveComponent Object Reference") (BoneName :type Name) (ShotFromDirection :type "Vector Structure") (InstigatedBy :type "Controller Object Reference") (DamageCauser :type "Actor Object Reference") (HitInfo :type "HitResult Structure (by ref)"))
  (bind (_bblockinghit _binitialoverlap _time _location _impactpoint _normal _impactnormal _physmat _hitactor _hitcomponent) (`GameplayStatics.BreakHitResult` HitInfo))
  (if (== _hitcomponent (`self.Target`))
    (bind _points (`self.HitPoints` _location))
    (`self.TargetHit` _points)
    (elif (== _hitcomponent (`self.ChainLeft01`))
      (`PhysicsConstraintComponent.BreakConstraint` (`self.Constr_ChainLeft01`))
      (elif (== _hitcomponent (`self.ChainLeft02`))
        (`PhysicsConstraintComponent.BreakConstraint` (`self.Constr_ChainLeft02`))
        (elif (== _hitcomponent (`self.ChainLeft03`))
          (`PhysicsConstraintComponent.BreakConstraint` (`self.Constr_ChainLeft03`))
          (elif (== _hitcomponent (`self.ChainLeft04`))
            (`PhysicsConstraintComponent.BreakConstraint` (`self.Constr_ChainLeft04`))
            (elif (== _hitcomponent (`self.ChainLeft05`))
              (`PhysicsConstraintComponent.BreakConstraint` (`self.Constr_ChainLeft05`))
              (elif (== _hitcomponent (`self.ChainLeft06`))
                (`PhysicsConstraintComponent.BreakConstraint` (`self.Constr_ChainLeft06`))
                (elif (== _hitcomponent (`self.ChainRight01`))
                  (`PhysicsConstraintComponent.BreakConstraint` (`self.Constr_ChainRight01`))
                  (elif (== _hitcomponent (`self.ChainRight02`))
                    (`PhysicsConstraintComponent.BreakConstraint` (`self.Constr_ChainRight02`))
                    (elif (== _hitcomponent (`self.ChainRight03`))
                      (`PhysicsConstraintComponent.BreakConstraint` (`self.Constr_ChainRight03`))
                      (elif (== _hitcomponent (`self.ChainRight04`))
                        (`PhysicsConstraintComponent.BreakConstraint` (`self.Constr_ChainRight04`))
                        (elif (== _hitcomponent (`self.ChainRight05`))
                          (`PhysicsConstraintComponent.BreakConstraint` (`self.Constr_ChainRight05`))
                          (elif (== _hitcomponent (`self.ChainRight06`))
                            (`PhysicsConstraintComponent.BreakConstraint` (`self.Constr_ChainRight06`))))))))))))))))

(fn `HitPoints`
  (params (Location :type "Vector Structure"))
  (returns (Points :type "Float (double-precision)"))
  (bind _returnvalue (`KismetMathLibrary.VSize` (- Location (`SceneComponent.K2_GetComponentLocation` (`self.Target`)))))
  (if (< _returnvalue 3.0)
    (return 10.0)
    (elif (< _returnvalue 10.0)
      (return 6.0)
      (elif (< _returnvalue 15.0)
        (return 5.0)
        (elif (< _returnvalue 15.0)
          (return 4.0)
          (elif (< _returnvalue 20.0)
            (return 3.0)
            (elif (< _returnvalue 30.0)
              (return 2.0)
              (elif (< _returnvalue 35.0)
                (return 1.0)
                (else
                  (return 0.0))))))))))

(fn `UserConstructionScript`)