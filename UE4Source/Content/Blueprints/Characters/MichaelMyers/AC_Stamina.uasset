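; Stamina component for the Michael Myers character that limits fast walking and attacking.
; A looping delay from BeginPlay refills stamina whenever it is not in use.
; FastWalking drains it and holds off refill with a retriggerable delay, while Attack removes a larger chunk.
; Tick locks both drains and clears CanFastWalk when stamina empties, until it recharges past a threshold.
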(event `self.ReceiveBeginPlay`
  ;[1 1 1] Recharge Stamina
  (if (not (`self.IsUsingStamina`)) :!label _label
    (set `self.CurrentStamina` (`KismetMathLibrary.FClamp` (+ (`self.CurrentStamina`) 1.0) 0.0 100.0)))
  (`KismetSystemLibrary.Delay` 0.1)
  (goto _label))

(event `self.ReceiveTick`
  (params (DeltaSeconds :type "Float (single-precision)"))
  (`|ExecutionSequence`
    (:`then_0`
      ;[1 1 1] Ran out of stamina
      (if (or (== (`self.CurrentStamina`) 0.0) (`self.Recharging`))
        (set `self.Recharging` true)
        (set `self.CanFastWalk` false)))
    (:`then_1`
      ;[1 1 1] Recharged high enough to preform actions again
      (if (>= (`self.CurrentStamina`) 20.0)
        (set `self.Recharging` false)
        (set `self.CanFastWalk` true)))))

(event `FastWalking`
  ;[1 1 1] Lose stamina from fast walk
  (if (not (`self.Recharging`))
    (set `self.IsUsingStamina` true)
    (set `self.CurrentStamina` (`KismetMathLibrary.FClamp` (- (`self.CurrentStamina`) 1.0) 0.0 100.0))
    (`KismetSystemLibrary.RetriggerableDelay` 0.5)
    (set `self.IsUsingStamina` false)))

(event `Attack`
  ;[1 1 1] Lose stamina from attack
  (if (not (`self.Recharging`))
    (set `self.CurrentStamina` (`KismetMathLibrary.FClamp` (- (`self.CurrentStamina`) 20.0) 0.0 100.0))))