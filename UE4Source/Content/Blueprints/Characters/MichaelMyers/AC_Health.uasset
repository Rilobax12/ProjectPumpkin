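; Health component in the Michael Myers character folder that tracks current health and triggers the owner's death.
; On BeginPlay it binds handlers to the Damage and Heal events, which subtract or add the passed amount and clamp the result to a fixed range.
; Tick polls for zero health and, through a DoOnce, prints a debug message and calls CallDeath on the owner's AC_Death component.
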(event `self.ReceiveTick`
  (params (DeltaSeconds :type "Float (single-precision)"))
  (if (<= (`self.CurrentHealth`) 0.0)
    (`/Engine/EditorBlueprintResources/StandardMacros.DoOnce` false
      (:`Completed`
        (`KismetSystemLibrary.PrintString` "Dead")
        (`/Game/Blueprints/Characters/MichaelMyers/AC_Death.Death` (`Actor.GetComponentByClass` (`self.GetOwner`) "/Game/Blueprints/Characters/MichaelMyers/AC_Death.AC_Death_C"))))))

(event `self.ReceiveBeginPlay`
  (add `self.Damage` (delegate `Damage_Event`))
  (add `self.Heal` (delegate `Heal_Event`)))

(event `Damage_Event` :!signature `self.Damage`
  (params (NewParam :type "Float (double-precision)"))
  (set `self.CurrentHealth` (`KismetMathLibrary.FClamp` (- (`self.CurrentHealth`) NewParam) 0.0 100.0)))

(event `Heal_Event` :!signature `self.Heal`
  (params (HealAmount :type "Float (double-precision)"))
  (set `self.CurrentHealth` (`KismetMathLibrary.FClamp` (+ (`self.CurrentHealth`) HealAmount) 0.0 100.0)))