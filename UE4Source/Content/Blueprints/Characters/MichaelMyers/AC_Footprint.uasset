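; Actor component that leaves footprint decals under its owner, revealed only during Michael Myers' Stalker ability.
; Left and right footprint events trace downward from the foot and spawn temporary decals, tracked in an array with visibility matching the current ability state.
; Stalker events bound from player 0's Michael character show all tracked prints, then hide them after the ability time or on cancel, removing invalid entries while iterating.
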(event `self.ReceiveBeginPlay`
  (bind _asedwin_als_michael (cast `/Game/Blueprints/Characters/MichaelMyers/edwinALS_Michael` (`GameplayStatics.GetPlayerCharacter` 0) :!pure true))
  (add `self.RightFootPrint` (delegate `RightFootPrint_Event`))
  (add `self.LeftFootPrint` (delegate `LeftFootPrint_Event`))
  (add `/Game/Blueprints/Characters/MichaelMyers/edwinALS_Michael.StalkerAbility` _asedwin_als_michael (delegate `StalkerAbility_Event`))
  (add `/Game/Blueprints/Characters/MichaelMyers/edwinALS_Michael.StalkerCancel` _asedwin_als_michael (delegate `StalkerCancel_Event`)))

(event `RightFootPrint_Event`
  (params (FootLocation :type "Vector Structure"))
  (set `self.FootLocation` FootLocation)
  ;[1 1 1] Make footprint
  (bind (_outhit _returnvalue) (`KismetSystemLibrary.LineTraceSingle` (`self.FootLocation`) (- (`self.FootLocation`) (0.0 0.0 100.0)) "TraceTypeQuery1" false (`|MakeArray` (`self.GetOwner`)) :!label _label))
  (if _returnvalue
    (bind _returnvalue_2 (`GameplayStatics.SpawnDecalAtLocation` "/Game/Materials/MAT_Asphalt_Patch_Decal.MAT_Asphalt_Patch_Decal" (10.0 10.0 10.0) (`.Location` (`GameplayStatics.BreakHitResult` _outhit)) (struct :`Pitch` -90.0) 30.0))
    (`KismetArrayLibrary.Array_Add` (`self.FootPrints`) _returnvalue_2)
    (`SceneComponent.SetVisibility` _returnvalue_2 (`self.IsVisible`) false)))

(event `LeftFootPrint_Event`
  (params (FootLocation :type "Vector Structure"))
  (set `self.FootLocation` FootLocation)
  (goto _label))

(event `StalkerAbility_Event`
  (params (AbilityTime :type "Float (double-precision)"))
  ;[1 1 1] Footprint visibility
  (set `self.IsVisible` true)
  (for _array_element (`self.FootPrints`)
    (`/Engine/EditorBlueprintResources/StandardMacros.IsValid` _array_element
      (:`Is Valid`
        (`SceneComponent.SetVisibility` _array_element true false))
      (:`Is Not Valid`
        (`KismetArrayLibrary.Array_RemoveItem` (`self.FootPrints`) _array_element))))
  (`KismetSystemLibrary.Delay` AbilityTime)
  (set `self.IsVisible` false :!label _label_2)
  (for _array_element_2 (`self.FootPrints`)
    (`/Engine/EditorBlueprintResources/StandardMacros.IsValid` _array_element_2
      (:`Is Valid`
        (`SceneComponent.SetVisibility` _array_element_2 false false))
      (:`Is Not Valid`
        (`KismetArrayLibrary.Array_RemoveItem` (`self.FootPrints`) _array_element_2)))))

(event `StalkerCancel_Event`
  ;[1 1 1] Footprint visibility
  (goto _label_2))