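; Actor component that briefly highlights its owner when Michael Myers' stalker ability fires.
; On BeginPlay it binds to the ability event on the player 0 character and adds or updates a blendable on the owner's PostProcessComponent.
; The event enables custom depth on the owner's first mesh component, presumably for a post-process outline, then disables it after a three-second delay.
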(event `self.ReceiveBeginPlay`
  (add `/Game/Blueprints/Characters/MichaelMyers/mixamoMichaelMyersControllerBP.StalkerAbility` (cast `/Game/Blueprints/Characters/MichaelMyers/mixamoMichaelMyersControllerBP` (`GameplayStatics.GetPlayerCharacter` 0) :!pure true) (delegate `StalkerAbility_Event`))
  (`PostProcessComponent.AddOrUpdateBlendable` (`Actor.GetComponentByClass` (`self.GetOwner`) "/Script/Engine.PostProcessComponent") null 1.0))

(event `StalkerAbility_Event`
  (bind _returnvalue (`Actor.GetComponentByClass` (`self.GetOwner`) "/Script/Engine.MeshComponent"))
  (`PrimitiveComponent.SetRenderCustomDepth` _returnvalue true)
  (`KismetSystemLibrary.Delay` 3.0)
  (`PrimitiveComponent.SetRenderCustomDepth` _returnvalue false))