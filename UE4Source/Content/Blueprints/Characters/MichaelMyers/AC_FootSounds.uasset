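; Actor component in the Michael Myers character folder that plays surface-dependent footstep sounds at foot impact points.
; On BeginPlay it binds to left and right foot events, which both feed a foot location into one shared downward line trace.
; The hit's physical material surface selects a random grass, wood or concrete sound to play at the hit location, with concrete as the fallback.
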(event `self.ReceiveBeginPlay`
  (add `self.LeftFoot` (delegate `LeftFoot_Event`))
  (add `self.RightFoot` (delegate `RightFoot_Event`)))

(event `LeftFoot_Event`
  (params (FootLocation :type "Vector Structure"))
  (set `self.SoundLocation` FootLocation)
  (bind (_outhit _returnvalue) (`KismetSystemLibrary.LineTraceSingle` (`self.SoundLocation`) (- (`self.SoundLocation`) (0.0 0.0 100.0)) "TraceTypeQuery1" false (`|MakeArray` (`self.GetOwner`)) :!label _label))
  (if _returnvalue
    (bind (_bblockinghit _binitialoverlap _time _distance _location _impactpoint _normal _impactnormal _physmat) (`GameplayStatics.BreakHitResult` _outhit))
    (switch `EPhysicalSurface` (`PhysicalMaterial.SurfaceType` _physmat)
      (:`SurfaceType_Default`
        (`GameplayStatics.PlaySoundAtLocation` (`|GetArrayItem` (`self.ConcreteFootstepSounds`) (`KismetMathLibrary.RandomIntegerInRange` 0 4)) _location (struct) 0.7 :!label _label_2))
      (:`SurfaceType1`
        (`GameplayStatics.PlaySoundAtLocation` (`|GetArrayItem` (`self.GrassFootstepSounds`) (`KismetMathLibrary.RandomIntegerInRange` 0 5)) _location (struct) 0.03))
      (:`SurfaceType2`
        (`GameplayStatics.PlaySoundAtLocation` (`|GetArrayItem` (`self.WoodFootstepSounds`) (`KismetMathLibrary.RandomIntegerInRange` 0 4)) _location (struct) 0.1))
      (:`SurfaceType3`
        (goto _label_2)))))

(event `RightFoot_Event`
  (params (NewParam :type "Vector Structure"))
  (set `self.SoundLocation` NewParam)
  (goto _label))