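; Backup of a character Blueprint event graph that adds a stamina-limited fast walk alongside rate-based controller look input.
; FastWalk press raises max walk speed and starts a looping timer that drains stamina, while release restores normal speed and starts a regeneration timer.
; Running out of stamina also drops to normal speed and begins regeneration, which stops once stamina reaches its maximum.
; Debug print nodes are left unconnected.
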(event `InputAxis|TurnRate`
  (params (AxisValue :type "Float (single-precision)"))
  ;[1 1 1] Walk Speed And Stamina System
  (`self.AddControllerYawInput` (* AxisValue (`self.BaseTurnRate`) (`GameplayStatics.GetWorldDeltaSeconds`))))

(event `DecreaseStamina`
  ;[1 1 1] Walk Speed And Stamina System
  (bind _output_get (set `self.CurrentStamina` (- (`self.CurrentStamina`) (`self.StaminaRate`))))
  (if (<= _output_get 0.0)
    (`KismetSystemLibrary.K2_ClearAndInvalidateTimerHandle` (stale `InputAction|FastWalk` _returnvalue))
    (set `CharacterMovementComponent.MaxWalkSpeed` 150.0 (`self.CharacterMovement`))
    (bind _returnvalue (`KismetSystemLibrary.K2_SetTimerDelegate` (delegate `IncreaseStamina`) 0.05 true))))

(event `InputAction|FastWalk`
  (params (Key :type "Key Structure"))
  (bind _charactermovement (`self.CharacterMovement`))
  ;[1 1 1] Walk Speed And Stamina System
  (:`Pressed`
    (set `CharacterMovementComponent.MaxWalkSpeed` 300.0 _charactermovement)
    (bind _returnvalue (`KismetSystemLibrary.K2_SetTimerDelegate` (delegate `DecreaseStamina`) 0.05 true))
    (`KismetSystemLibrary.K2_ClearAndInvalidateTimerHandle` (stale `InputAction|FastWalk` _returnvalue_2))
    (`KismetSystemLibrary.K2_ClearAndInvalidateTimerHandle` (stale `DecreaseStamina` _returnvalue)))
  (:`Released`
    (set `CharacterMovementComponent.MaxWalkSpeed` 150.0 _charactermovement)
    (bind _returnvalue_2 (`KismetSystemLibrary.K2_SetTimerDelegate` (delegate `IncreaseStamina`) 0.05 true))
    (`KismetSystemLibrary.K2_ClearAndInvalidateTimerHandle` _returnvalue)))

(event `IncreaseStamina`
  ;[1 1 1] Walk Speed And Stamina System
  (bind _output_get (set `self.CurrentStamina` (+ (`self.CurrentStamina`) (`self.StaminaRate`))))
  (if (>= _output_get (`self.MaxStamina`))
    (`KismetSystemLibrary.K2_ClearAndInvalidateTimerHandle` (stale `InputAction|FastWalk` _returnvalue_2))
    (`KismetSystemLibrary.K2_ClearAndInvalidateTimerHandle` (stale `DecreaseStamina` _returnvalue))))

(event `InputAxis|LookUpRate`
  (params (AxisValue :type "Float (single-precision)"))
  ;[1 1 1] Walk Speed And Stamina System
  (`self.AddControllerPitchInput` (* AxisValue (`self.BaseLookUpRate`) (`GameplayStatics.GetWorldDeltaSeconds`))))

(fn `UserConstructionScript`)