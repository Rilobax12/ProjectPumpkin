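; BP_QTE_Cams is a camera rig for quick time events that switches between preset scenic cameras by index.
; The construction script builds a camera array matching the Enum_CameraList order, with index 0 left empty for None.
; Manual_Cam deactivates all cameras, then activates the requested one, falling back to the last valid camera, and sets ValidCam.
; Optional Player and Opposite preview meshes are removed at construction unless ShowMesh is set, and always on BeginPlay.
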(event `self.ReceiveBeginPlay`
  (bind _player (`self.player`))
  (bind _opposite (`self.opposite`))
  ;[1 1 1] destroy example mesh if you forgot to do it by bool
  (`/Engine/EditorBlueprintResources/StandardMacros.IsValid` _player
    (:`Is Valid`
      (`ActorComponent.K2_DestroyComponent` _player))
    (:`Is Not Valid`
      _))
  (`/Engine/EditorBlueprintResources/StandardMacros.IsValid` _opposite
    (:`Is Valid`
      (`ActorComponent.K2_DestroyComponent` _opposite))))

(event `DeactivateCams`
  ;[1 0 0] deactivates all cameras before setting active one
  (for _array_element (`self.CameraArray`)
    (`/Engine/EditorBlueprintResources/StandardMacros.IsValid` _array_element
      (:`Is Valid`
        (`ActorComponent.SetActive` _array_element false false)))))

(event `Manual_Cam`
  (params (Index :type Integer))
  (bind _lastvalidcam (`self.LastValidCam`))
  (bind _item (`KismetArrayLibrary.Array_Get` (`self.CameraArray`) Index))
  ;[0.2661 1 0.3223] sets manual cams from struct array
  (`self.DeactivateCams`)
  (`/Engine/EditorBlueprintResources/StandardMacros.IsValid` _item ; index (0) is always invalid because its None from enum_CameraList\nso latest valid camera will remain active at None
    (:`Is Valid`
      (`ActorComponent.SetActive` _item true false)
      (set `self.LastValidCam` _item) ; latest valid cam
    )
    (:`Is Not Valid`
      (`/Engine/EditorBlueprintResources/StandardMacros.IsValid` _lastvalidcam ; gets if last valid cam is valid
        (:`Is Valid`
          (`ActorComponent.SetActive` _lastvalidcam true false) ; this activates at "None"
        ))))
  (set `self.ValidCam` true) ; sets that cam is valid so switch will happen
)

(event `CreateCameraList`
  ;[0.3241 0.3008 1] calls by construct
  (set `self.CameraArray` (`|MakeArray` null (`self.C_L1`) (`self.C_L2`) (`self.C_L3`) (`self.C_R1`) (`self.C_R2`) (`self.C_R3`) (`self.C_T1`) (`self.C_T2`) (`self.C_T3`) (`self.C_C1`) null)) ; the array index list is equal to enum index list for manual scenic camera's
)

(fn `UserConstructionScript`
  ;[1 1 1] show optional mesh and create camera list
  (if (not (`self.ShowMesh?`))
    (`ActorComponent.K2_DestroyComponent` (`self.opposite`))
    (`ActorComponent.K2_DestroyComponent` (`self.player`)))
  (`self.CreateCameraList`))